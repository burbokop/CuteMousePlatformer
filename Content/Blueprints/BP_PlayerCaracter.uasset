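; Player character Blueprint for side-on flipbook movement, with run, idle and jump animations.
; BeginPlay adds the default Enhanced Input mapping context, and movement input drives the character along its forward vector while yawing the sprite to face the travel direction.
; A state enum keeps run and idle from overriding the non-looping jump flipbook.
; After a jump, a delay loop polls vertical velocity until zero, then restores the grounded state and looping idle.
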(event Input|EnhancedActionEvents|EnhancedInputActionIA_Movement
  (params (ActionValue :type Float%20%28double-precision%29) (ElapsedSeconds :type Float%20%28double-precision%29) (TriggeredSeconds :type Float%20%28double-precision%29) (InputAction :type Input%20Action%20Object%20Reference :default "/Game/Blueprints/IA_Movement.IA_Movement"))
  (bind _sprite (Variables|Default|GetSprite))
  (bind _state (Variables|Default|GetState))
  (bind _returnvalue (Utilities|Enum|Equal(Enum) _state "NewEnumerator0"))
  (:Triggered
    (Pawn|Input|AddMovementInput (Transformation|GetActorForwardVector) (* ActionValue 0.2) false)
    (Transformation|SetWorldRotation (Variables|Default|GetSprite) (Math|Rotator|MakeRotator 0.0 0.0 (select (> ActionValue 0.0) 0.0 -1.8e+02)) false false)
    (if _returnvalue
      (Sprite|SetFlipbook _sprite "/Game/Assets/Run2.Run2")))
  (:Completed
    (if _returnvalue
      (Sprite|SetFlipbook _sprite "/Game/Assets/Idle.Idle"))))

(event Input|EnhancedActionEvents|EnhancedInputActionIA_Jump
  (params (ActionValue :type Boolean) (ElapsedSeconds :type Float%20%28double-precision%29) (TriggeredSeconds :type Float%20%28double-precision%29) (InputAction :type Input%20Action%20Object%20Reference :default "/Game/Blueprints/IA_Jump.IA_Jump"))
  (bind _sprite (Variables|Default|GetSprite))
  (Variables|Default|SetState "NewEnumerator1")
  (Character|Jump)
  (Sprite|SetFlipbook (Variables|Default|GetSprite) "/Game/Assets/Jump2.Jump2")
  (Components|Timeline|SetLooping (Variables|Default|GetSprite) false)
  (Utilities|FlowControl|Delay 0.2)
  (if (== (.z (Transformation|GetVelocity)) 0.0) :!label _label
    (Variables|Default|SetState "NewEnumerator0")
    (Sprite|SetFlipbook _sprite "/Game/Assets/Idle.Idle")
    (Components|Timeline|SetLooping _sprite true)
    (Audio|Components|Audio|Play _sprite)
    (else
      (Utilities|FlowControl|Delay 0.05)
      (goto _label))))

(event EventBeginPlay
  (bind _asbp_player_controller (Utilities|Casting|CastToBP_PlayerController (Pawn|GetController)))
  (Input|AddMappingContext (PlayerController|LocalPlayerSubsystems|GetEnhancedInputLocalPlayerSubsystem _asbp_player_controller) "/Game/Blueprints/IMC_Default.IMC_Default" 0 "(bIgnoreAllPressedKeysUntilRelease=True,bForceImmediately=False,bNotifyUserSettings=False)"))

(event Collision|EventActorBeginOverlap
  (params (OtherActor :type Actor%20Object%20Reference)))

(event EventTick
  (params (DeltaSeconds :type Float%20%28single-precision%29)))

(fn ConstructionScript)