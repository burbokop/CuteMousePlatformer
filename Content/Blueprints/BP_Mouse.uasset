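; BP_Mouse is the player-controlled 2D flipbook mouse character, which runs, sneaks and jumps.
; Enhanced Input drives movement along the forward vector, scales it by sneak or run speed, and flips the sprite by yaw.
; A state enum gates flipbook changes.
; Jumps and Tick-detected falls share a delay loop that polls IsFalling until landing, then restores the idle state.
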(event Input|EnhancedActionEvents|EnhancedInputActionIA_Movement
  (params (ActionValue :type Float%20%28double-precision%29) (ElapsedSeconds :type Float%20%28double-precision%29) (TriggeredSeconds :type Float%20%28double-precision%29) (InputAction :type Input%20Action%20Object%20Reference :default "/Game/Blueprints/IA_Movement.IA_Movement"))
  (bind _sprite (Variables|Default|GetSprite))
  (bind _state (Variables|Default|GetState))
  (bind _returnvalue (Utilities|Enum|Equal(Enum) _state "NewEnumerator0"))
  (:Triggered
    (Pawn|Input|AddMovementInput (Transformation|GetActorForwardVector) (* ActionValue (select (Variables|Default|GetSneaking) (Variables|Default|GetSneak%20speed) (Variables|Default|GetRun%20speed))) false)
    (Transformation|SetWorldRotation (Variables|Default|GetSprite) (Math|Rotator|MakeRotator 0.0 0.0 (select (> ActionValue 0.0) 0.0 -1.8e+02)) false false)
    (if _returnvalue
      (if (Variables|Default|GetSneaking)
        (Sprite|SetFlipbook _sprite "/Game/Assets/Flipbooks/Walk.Walk")
        (else
          (Sprite|SetFlipbook _sprite "/Game/Assets/Flipbooks/Run.Run")))))
  (:Completed
    (if _returnvalue
      (Sprite|SetFlipbook _sprite "/Game/Assets/Flipbooks/Idle.Idle"))))

(event Input|EnhancedActionEvents|EnhancedInputActionIA_Jump
  (params (ActionValue :type Boolean) (ElapsedSeconds :type Float%20%28double-precision%29) (TriggeredSeconds :type Float%20%28double-precision%29) (InputAction :type Input%20Action%20Object%20Reference :default "/Game/Blueprints/IA_Jump.IA_Jump"))
  (bind _sprite (Variables|Default|GetSprite))
  (if (Utilities|Enum|Equal(Enum) (Variables|Default|GetState) "NewEnumerator0")
    (Variables|Default|SetState "NewEnumerator1")
    (Character|Jump)
    (Sprite|SetFlipbook (Variables|Default|GetSprite) "/Game/Assets/Flipbooks/Jump.Jump")
    (Components|Timeline|SetLooping (Variables|Default|GetSprite) false)
    (Utilities|FlowControl|Delay 0.2)
    (if (AI|Components|NavMovement|IsFalling (Variables|Character|GetCharacterMovement)) :!label _label
      (Utilities|FlowControl|Delay 0.05)
      (goto _label)
      (else
        (Variables|Default|SetState "NewEnumerator0")
        (Sprite|SetFlipbook _sprite "/Game/Assets/Flipbooks/Idle.Idle")
        (Components|Timeline|SetLooping _sprite true)
        (Audio|Components|Audio|Play _sprite)))))

(event Input|EnhancedActionEvents|EnhancedInputActionIA_Sneak
  (params (ActionValue :type Boolean) (ElapsedSeconds :type Float%20%28double-precision%29) (TriggeredSeconds :type Float%20%28double-precision%29) (InputAction :type Input%20Action%20Object%20Reference :default "/Game/Blueprints/IA_Sneak.IA_Sneak"))
  (bind _state (Variables|Default|GetState))
  (bind _sprite (Variables|Default|GetSprite))
  (bind _returnvalue (Utilities|Enum|Equal(Enum) _state "NewEnumerator0"))
  (:Triggered
    (Variables|Default|SetSneaking true)
    (if _returnvalue
      (Sprite|SetFlipbook _sprite "/Game/Assets/Flipbooks/Walk.Walk")))
  (:Completed
    (Variables|Default|SetSneaking false)
    (if _returnvalue
      (Sprite|SetFlipbook _sprite "/Game/Assets/Flipbooks/Run.Run"))))

(event EventBeginPlay
  (bind _asbp_player_controller (Utilities|Casting|CastToBP_PlayerController (Pawn|GetController)))
  (Input|AddMappingContext (PlayerController|LocalPlayerSubsystems|GetEnhancedInputLocalPlayerSubsystem _asbp_player_controller) "/Game/Blueprints/IMC_Default.IMC_Default" 0 "(bIgnoreAllPressedKeysUntilRelease=True,bForceImmediately=False,bNotifyUserSettings=False)"))

(event Collision|EventActorBeginOverlap
  (params (OtherActor :type Actor%20Object%20Reference)))

(event EventTick
  (params (DeltaSeconds :type Float%20%28single-precision%29))
  (bind _sprite (Variables|Default|GetSprite))
  (if (and (AI|Components|NavMovement|IsFalling (Variables|Character|GetCharacterMovement)) (Utilities|Enum|Equal(Enum) (Variables|Default|GetState) "NewEnumerator0"))
    (Variables|Default|SetState "NewEnumerator3")
    (Sprite|SetFlipbook (Variables|Default|GetSprite) "/Game/Assets/Flipbooks/Fall.Fall")
    (Components|Timeline|SetLooping (Variables|Default|GetSprite) false)
    (Utilities|FlowControl|Delay 0.2)
    (if (AI|Components|NavMovement|IsFalling (Variables|Character|GetCharacterMovement)) :!label _label
      (Utilities|FlowControl|Delay 0.05)
      (goto _label)
      (else
        (Variables|Default|SetState "NewEnumerator0")
        (Sprite|SetFlipbook _sprite "/Game/Assets/Flipbooks/Idle.Idle")
        (Components|Timeline|SetLooping _sprite true)
        (Audio|Components|Audio|Play _sprite)))))

(fn ConstructionScript)