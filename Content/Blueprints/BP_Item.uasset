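; BP_Item is a sprite-based item actor that shows an outline while a BP_Mouse actor is within its collision sphere.
; On BeginPlay it applies one configurable sprite to both the main and outline sprite components and sets the sphere radius.
; BeginPlay and overlap begin/end events set outline visibility by querying the sphere for overlapping BP_Mouse actors.
; An alternative material-swap highlight remains in the graph but is unconnected.
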(event EventBeginPlay
  (bind _sprite (Variables|Default|GetSprite))
  (Rendering|Components|Sprite|SetSprite (Variables|Default|GetMainSprite) _sprite)
  (Rendering|Components|Sprite|SetSprite (Variables|Default|GetOutlineSprite) _sprite)
  (Components|Sphere|SetSphereRadius (Variables|Default|GetCollisionSphere) (Variables|Default|GetCollision%20Radius) true)
  (Rendering|SetVisibility (Variables|Default|GetOutlineSprite) (!= (Utilities|Array|Length (Collision|GetOverlappingActors (Variables|Default|GetCollisionSphere) "/Game/Blueprints/BP_Mouse.BP_Mouse_C" :!class /Script/Engine.PrimitiveComponent)) 0) false))

(event Collision|EventActorBeginOverlap
  (params (OtherActor :type Actor%20Object%20Reference))
  (Rendering|SetVisibility (Variables|Default|GetOutlineSprite) (!= (Utilities|Array|Length (Collision|GetOverlappingActors (Variables|Default|GetCollisionSphere) "/Game/Blueprints/BP_Mouse.BP_Mouse_C" :!class /Script/Engine.PrimitiveComponent)) 0) false))

(event EventTick
  (params (DeltaSeconds :type Float%20%28single-precision%29)))

(event Collision|EventActorEndOverlap
  (params (OtherActor :type Actor%20Object%20Reference))
  (Rendering|SetVisibility (Variables|Default|GetOutlineSprite) (!= (Utilities|Array|Length (Collision|GetOverlappingActors (Variables|Default|GetCollisionSphere) "/Game/Blueprints/BP_Mouse.BP_Mouse_C" :!class /Script/Engine.PrimitiveComponent)) 0) false))

(fn ConstructionScript)